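; Drivable Orion car pawn with throttle, steering, handbrake, first-press engine start, brake-light swap, random body paint, flip reset and hold-for-slow-motion.
; Tick feeds RPM to engine audio and traces downward to detect ground and Landscape versus track.
; Sideways velocity triggers tyre decals on track and Landscape driving leaves dirt decals, aligned to wheel velocity.
; The rear-drift flag fades skid audio, and hits spawn sparks with a brief light flash.
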(event Custom|Extra%20Tick%202)

(event Custom|Extra%20Tick%201
  (bind _road_skid_ext (Variables|Default|Getroad_skid_ext))
  (if (Variables|Default|GetDrifting?)
    (Utilities|FlowControl|DoOnce false :!label _label
      (:Completed
        (Audio|Components|Audio|FadeIn _road_skid_ext 1.0 0.2 0.0 "Linear" :!class /Script/Engine.AudioComponent)
        (goto _label_2 Reset)))
    (else
      (Utilities|FlowControl|DoOnce false :!label _label_2
        (:Completed
          (Audio|Components|Audio|FadeOut _road_skid_ext 0.5 0.0 "Linear" :!class /Script/Engine.AudioComponent)
          (goto _label Reset))))))

(event EventBeginPlay
  (bind _mesh (Variables|Character|GetMesh))
  (switch int (Math|Random|RandomIntegerinRange 0 3)
    (:0
      (Rendering|Material|SetMaterial _mesh 17 "/Game/ColourMats/White_Gloss.White_Gloss"))
    (:1
      (Rendering|Material|SetMaterial _mesh 17 "/Game/ColourMats/Black_Gloss.Black_Gloss"))
    (:2
      (Rendering|Material|SetMaterial _mesh 17 "/Game/ColourMats/Gray_Gloss.Gray_Gloss"))
    (:3
      (Rendering|Material|SetMaterial _mesh 17 "/Game/ColourMats/Dark_Gray_Gloss.Dark_Gray_Gloss"))))

(event Collision|EventActorBeginOverlap
  (params (OtherActor :type Actor%20Object%20Reference)))

(event EventTick
  (params (DeltaSeconds :type Float%20%28single-precision%29))
  (bind _returnvalue (Transformation|GetActorRotation))
  (bind _returnvalue_2 (Transformation|GetVelocity))
  (bind _returnvalue_3 (Transformation|GetActorRotation))
  (bind _returnvalue_4 (Transformation|GetVelocity))
  (bind _left_wheel_location_arrow (Variables|Default|GetLeft%20Wheel%20Location%20Arrow))
  (bind _bodycenter (Variables|Default|GetBodyCenter))
  (bind _left_wheel_location_arrow_2 (Variables|Default|GetLeft%20Wheel%20Location%20Arrow))
  (bind _right_wheel_location_arrow (Variables|Default|GetRight%20Wheel%20Location%20Arrow))
  (bind _left_wheel_location_arrow1 (Variables|Default|GetLeft%20Wheel%20Location%20Arrow1))
  (bind _right_wheel_location_arrow1 (Variables|Default|GetRight%20Wheel%20Location%20Arrow1))
  (bind _right_wheel_location_arrow_2 (Variables|Default|GetRight%20Wheel%20Location%20Arrow))
  (bind _left_wheel_location_arrow1_2 (Variables|Default|GetLeft%20Wheel%20Location%20Arrow1))
  (bind _right_wheel_location_arrow1_2 (Variables|Default|GetRight%20Wheel%20Location%20Arrow1))
  (bind _returnvalue_5 (Transformation|GetWorldLocation _right_wheel_location_arrow1))
  (bind _returnvalue_6 (Transformation|GetWorldLocation _left_wheel_location_arrow_2))
  (bind _returnvalue_7 (Transformation|GetWorldLocation _right_wheel_location_arrow))
  (bind _returnvalue_8 (Transformation|GetWorldLocation _left_wheel_location_arrow1))
  (bind _returnvalue_9 (Transformation|GetWorldLocation _right_wheel_location_arrow_2))
  (bind _returnvalue_10 (Math|Vector|GetRightVector _returnvalue))
  (bind _returnvalue_11 (Math|Vector|GetRightVector _returnvalue_3))
  (bind _returnvalue_12 (Transformation|GetWorldLocation _bodycenter))
  (bind _returnvalue_13 (Transformation|GetWorldLocation _left_wheel_location_arrow))
  (bind _returnvalue_14 (Transformation|GetWorldLocation _left_wheel_location_arrow1_2))
  (bind _returnvalue_15 (Transformation|GetWorldLocation _right_wheel_location_arrow1_2))
  (bind _returnvalue_16 (Math|Vector|DotProduct _returnvalue_10 _returnvalue_2))
  (bind _returnvalue_17 (Math|Vector|DotProduct _returnvalue_11 _returnvalue_4))
  (CallFunction|ExtraTick1)
  (CallFunction|ExtraTick2)
  (bind (_outhit _returnvalue_18) (Collision|LineTraceByChannel _returnvalue_12 (- _returnvalue_12 "0, 0,100.000000") "TraceTypeQuery1" true 0 "None"))
  (Utilities|FlowControl|Sequence
    (:then_0
      (Variables|Default|SetOnGround? _returnvalue_18)
      (bind _output_get (Variables|Default|SetDeltaSeconds DeltaSeconds))
      (Audio|Parameter|SetFloatParameter (Variables|Default|GetAuto) "RPM" (Class|WheeledVehicleMovementComponent|GetEngineRotationSpeed (Variables|Default|GetVehicleMovement)) :!class /Script/Engine.AudioComponent)
      (Variables|Default|SetSpeed (Math|Float|Floor (Math|Float|Absolute(Float) (* (Class|WheeledVehicleMovementComponent|GetForwardSpeed (Variables|Default|GetVehicleMovement)) 0.036))))
      (if (Variables|Default|GetOnGround?)
        (Utilities|FlowControl|Delay _output_get)
        (Utilities|FlowControl|Sequence
          (:then_0
            (if (or (> _returnvalue_16 5e+02) (< _returnvalue_16 -5e+02))
              (if (Variables|Default|GetOnTrack?)
                ;[1 1 1] Drift marks
                ;;[1 1 1] Left Wheel
                (if (> (Class|WheeledVehicleMovementComponent|GetForwardSpeed (Variables|Default|GetVehicleMovement)) 2.0)
                  (bind _returnvalue_19 (Class|PrimitiveComponent|GetPhysicsLinearVelocityatPoint (Variables|Character|GetMesh) _returnvalue_13 "None"))
                  (Rendering|Decal|SpawnDecalatLocation "/Game/FX/Tyremark_Mat.Tyremark_Mat" (Math|Vector|MakeVector (Math|Float|MapRangeClamped (Math|Conversions|ToFloat(Integer) (Variables|Default|GetSpeed)) 0.0 3e+02 3e+01 7e+01) 1e+01 2e+01) _returnvalue_13 (Math|Rotator|MakeRotfromX (Math|Vector|Normalize (Math|Vector|ProjectVectorontoPlane _returnvalue_19 (Math|Vector|GetUpVector (Variables|Character|GetMesh))))) 5.0)
                  ;;[1 1 1] Right Wheel
                  (bind _returnvalue_20 (Class|PrimitiveComponent|GetPhysicsLinearVelocityatPoint (Variables|Character|GetMesh) _returnvalue_7 "None"))
                  (Rendering|Decal|SpawnDecalatLocation "/Game/FX/Tyremark_Mat.Tyremark_Mat" (Math|Vector|MakeVector (Math|Float|MapRangeClamped (Math|Conversions|ToFloat(Integer) (Variables|Default|GetSpeed)) 0.0 3e+02 3e+01 7e+01) 1e+01 2e+01) _returnvalue_7 (Math|Rotator|MakeRotfromX (Math|Vector|Normalize (Math|Vector|ProjectVectorontoPlane _returnvalue_20 (Math|Vector|GetUpVector (Variables|Character|GetMesh))))) 5.0)
                  (Variables|Default|SetDrifting? true))
                (else
                  (Variables|Default|SetDrifting? false)))
              (else
                (Variables|Default|SetDrifting? false))))
          (:then_1
            ;[1 1 1] Front Wheels
            ;;[1 1 1] Left Wheel
            (if (or (> _returnvalue_17 1e+03) (< _returnvalue_17 -1e+03))
              (if (Variables|Default|GetOnTrack?)
                (bind _returnvalue_21 (Class|PrimitiveComponent|GetPhysicsLinearVelocityatPoint (Variables|Character|GetMesh) _returnvalue_14 "None"))
                (Rendering|Decal|SpawnDecalatLocation "/Game/FX/Tyremark_Mat.Tyremark_Mat" (Math|Vector|MakeVector (Math|Float|MapRangeClamped (Math|Conversions|ToFloat(Integer) (Variables|Default|GetSpeed)) 0.0 2.5e+02 3e+01 7e+01) 1e+01 2e+01) _returnvalue_14 (Math|Rotator|MakeRotfromX (Math|Vector|Normalize (Math|Vector|ProjectVectorontoPlane _returnvalue_21 (Math|Vector|GetUpVector (Variables|Character|GetMesh))))) 5.0)
                ;;[1 1 1] Right Wheel
                (bind _returnvalue_22 (Class|PrimitiveComponent|GetPhysicsLinearVelocityatPoint (Variables|Character|GetMesh) _returnvalue_15 "None"))
                (Rendering|Decal|SpawnDecalatLocation "/Game/FX/Tyremark_Mat.Tyremark_Mat" (Math|Vector|MakeVector (Math|Float|MapRangeClamped (Math|Conversions|ToFloat(Integer) (Variables|Default|GetSpeed)) 0.0 2.5e+02 3e+01 7e+01) 1e+01 2e+01) _returnvalue_15 (Math|Rotator|MakeRotfromX (Math|Vector|Normalize (Math|Vector|ProjectVectorontoPlane _returnvalue_22 (Math|Vector|GetUpVector (Variables|Character|GetMesh))))) 5.0)))))
        (else
          (Variables|Default|SetDrifting? false))))
    (:then_1
      (if (== (.PhysMat (Collision|BreakHitResult _outhit)) "/Game/Misc/Landscape.Landscape")
        (Variables|Default|SetOnTrack? false)
        (if (Variables|Default|GetOnGround?)
          ;[1 1 1] Dirt marks
          ;;[1 1 1] Left Wheel
          (if (or (> (Class|WheeledVehicleMovementComponent|GetForwardSpeed (Variables|Default|GetVehicleMovement)) 1e+01) (< (Class|WheeledVehicleMovementComponent|GetForwardSpeed (Variables|Default|GetVehicleMovement)) -5.0))
            (bind _returnvalue_23 (Class|PrimitiveComponent|GetPhysicsLinearVelocityatPoint (Variables|Character|GetMesh) _returnvalue_6 "None"))
            (Rendering|Decal|SpawnDecalatLocation "/Game/FX/Dirt_Tyremark_Mat.Dirt_Tyremark_Mat" (Math|Vector|MakeVector 7e+01 (Math|Float|MapRangeClamped (Math|Conversions|ToFloat(Integer) (Variables|Default|GetSpeed)) 0.0 2.5e+02 1e+01 25.0) 2e+01) _returnvalue_6 (Math|Rotator|MakeRotfromX (Math|Vector|Normalize (Math|Vector|ProjectVectorontoPlane _returnvalue_23 (Math|Vector|GetUpVector (Variables|Character|GetMesh))))) 5.0)
            ;;[1 1 1] Right Wheel
            (bind _returnvalue_24 (Class|PrimitiveComponent|GetPhysicsLinearVelocityatPoint (Variables|Character|GetMesh) _returnvalue_9 "None"))
            (Rendering|Decal|SpawnDecalatLocation "/Game/FX/Dirt_Tyremark_Mat.Dirt_Tyremark_Mat" (Math|Vector|MakeVector 7e+01 (Math|Float|MapRangeClamped (Math|Conversions|ToFloat(Integer) (Variables|Default|GetSpeed)) 0.0 2.5e+02 1e+01 25.0) 2e+01) _returnvalue_9 (Math|Rotator|MakeRotfromX (Math|Vector|Normalize (Math|Vector|ProjectVectorontoPlane _returnvalue_24 (Math|Vector|GetUpVector (Variables|Character|GetMesh))))) 1e+01)
            (bind _returnvalue_25 (Class|PrimitiveComponent|GetPhysicsLinearVelocityatPoint (Variables|Character|GetMesh) _returnvalue_8 "None"))
            (Rendering|Decal|SpawnDecalatLocation "/Game/FX/Dirt_Tyremark_Mat.Dirt_Tyremark_Mat" (Math|Vector|MakeVector 7e+01 (Math|Float|MapRangeClamped (Math|Conversions|ToFloat(Integer) (Variables|Default|GetSpeed)) 0.0 2.5e+02 1e+01 25.0) 2e+01) _returnvalue_8 (Math|Rotator|MakeRotfromX (Math|Vector|Normalize (Math|Vector|ProjectVectorontoPlane _returnvalue_25 (Math|Vector|GetUpVector (Variables|Character|GetMesh))))) 5.0)
            (bind _returnvalue_26 (Class|PrimitiveComponent|GetPhysicsLinearVelocityatPoint (Variables|Character|GetMesh) _returnvalue_5 "None"))
            (Rendering|Decal|SpawnDecalatLocation "/Game/FX/Dirt_Tyremark_Mat.Dirt_Tyremark_Mat" (Math|Vector|MakeVector 7e+01 (Math|Float|MapRangeClamped (Math|Conversions|ToFloat(Integer) (Variables|Default|GetSpeed)) 0.0 2.5e+02 1e+01 25.0) 2e+01) _returnvalue_5 (Math|Rotator|MakeRotfromX (Math|Vector|Normalize (Math|Vector|ProjectVectorontoPlane _returnvalue_26 (Math|Vector|GetUpVector (Variables|Character|GetMesh))))) 1e+01)))
        (else
          (Variables|Default|SetOnTrack? true))))))

(event Collision|EventHit
  (params (MyComp :type Primitive%20Component%20Object%20Reference) (Other :type Actor%20Object%20Reference) (OtherComp :type Primitive%20Component%20Object%20Reference) (bSelfMoved :type Boolean) (HitLocation :type Vector :default "0, 0, 0") (HitNormal :type Vector :default "0, 0, 0") (NormalImpulse :type Vector :default "0, 0, 0") (Hit :type Hit%20Result%20Structure%20%28by%20ref%29))
  (bind _pointlight (Variables|Default|GetPointLight))
  (if (> (Class|WheeledVehicleMovementComponent|GetForwardSpeed (Variables|Default|GetVehicleMovement)) 2.0)
    (if (> (Variables|Default|GetSpeed) 50)
      (Effects|SpawnEmitteratLocation "/Game/FX/P_Sparks.P_Sparks" HitLocation "0, 0, 0" "0.500000,0.500000,0.500000")
      (else
        (Effects|SpawnEmitteratLocation "/Game/FX/P_Sparks.P_Sparks" "0, 0, 0")))
    (Development|SetHiddeninGame _pointlight false false)
    (Transformation|SetWorldLocation _pointlight HitLocation false false)
    (Utilities|FlowControl|Delay 0.2)
    (Development|SetHiddeninGame _pointlight true false)))

(event Input|ActionEvents|InputActionHandbrake
  (params (Key :type Key%20Structure :default "None"))
  ;[1 1 1] Input
  (:Pressed
    (Class|WheeledVehicleMovementComponent|SetHandbrakeInput (Variables|Default|GetVehicleMovement) true))
  (:Released
    (Class|WheeledVehicleMovementComponent|SetHandbrakeInput (Variables|Default|GetVehicleMovement) false)))

(event Input|ActionEvents|InputActionBrake
  (params (Key :type Key%20Structure :default "None"))
  (bind _mesh (Variables|Character|GetMesh))
  ;[1 1 1] Brakelights
  (:Pressed
    (Rendering|Material|SetMaterial _mesh 6 "/Game/ColourMats/Red_Glow.Red_Glow"))
  (:Released
    (Rendering|Material|SetMaterial _mesh 6 "/Game/VehicleAdv/Materials/MaterialInstances/SolidRed.SolidRed")))

(event Input|AxisEvents|InputAxisLookUp
  (params (AxisValue :type Float%20%28single-precision%29))
  ;[1 1 1] Camera
  (Transformation|AddRelativeRotation (Variables|Default|GetSpringArm) (Math|Rotator|MakeRotator 0.0 0.0 0.0) false false))

(event Input|AxisEvents|InputAxisLookRight
  (params (AxisValue :type Float%20%28single-precision%29))
  ;[1 1 1] Camera
  (Transformation|AddRelativeRotation (Variables|Default|GetSpringArm) (Math|Rotator|MakeRotator 0.0 0.0 0.0) false false))

(event Input|AxisEvents|InputAxisMoveForward
  (params (AxisValue :type Float%20%28single-precision%29))
  ;[1 1 1] Input
  (if (Variables|Default|GetCarStarted)
    (Class|WheeledVehicleMovementComponent|SetThrottleInput (Variables|Default|GetVehicleMovement) AxisValue)))

(event Input|AxisEvents|InputAxisMoveRight
  (params (AxisValue :type Float%20%28single-precision%29))
  ;[1 1 1] Input
  (Class|WheeledVehicleMovementComponent|SetSteeringInput (Variables|Default|GetVehicleMovement) AxisValue))

(event Input|KeyboardEvents|Enter
  (params (Key :type Key%20Structure :default "None"))
  (:Pressed
    (Utilities|Time|SetGlobalTimeDilation 0.2))
  (:Released
    (Utilities|Time|SetGlobalTimeDilation 1.0)))

(event Input|KeyboardEvents|W
  (params (Key :type Key%20Structure :default "None"))
  (:Pressed
    (Utilities|FlowControl|DoOnce false
      (:Completed
        (Audio|PlaySoundatLocation "/Game/Misc/CarStart.CarStart" (Transformation|GetActorLocation) "0, 0, 0" 2.0 1.0 0.0 "/Game/VehicleAdv/Sound/Engine_att.Engine_att" 0 0)
        (Utilities|FlowControl|Delay 0.7)
        (Components|Activation|Activate (Variables|Default|GetAuto) false)
        (Utilities|FlowControl|Delay 0.2)
        (Variables|Default|SetCarStarted true)))))

(event Input|KeyboardEvents|S
  (params (Key :type Key%20Structure :default "None"))
  (:Pressed
    (Utilities|FlowControl|DoOnce false
      (:Completed
        (Audio|PlaySoundatLocation "/Game/Misc/CarStart.CarStart" (Transformation|GetActorLocation) "0, 0, 0" 2.0 1.0 0.0 "/Game/VehicleAdv/Sound/Engine_att.Engine_att" 0 0)
        (Utilities|FlowControl|Delay 0.7)
        (Components|Activation|Activate (Variables|Default|GetAuto) false)
        (Utilities|FlowControl|Delay 0.2)
        (Variables|Default|SetCarStarted true)))))

(event Input|KeyboardEvents|R
  (params (Key :type Key%20Structure :default "None"))
  (bind _returnvalue (Transformation|GetActorRotation))
  (bind (_roll _pitch _yaw) (Math|Rotator|BreakRotator _returnvalue))
  (:Pressed
    (if (Variables|Default|GetCanReset?)
      (Transformation|AddActorWorldOffset "0, 0,100.000000" false true)
      (Transformation|SetActorRotation (Math|Rotator|MakeRotator 0.0 _pitch _yaw) true)
      (Variables|Default|SetCanReset? false)
      (Utilities|FlowControl|Delay 1.5)
      (Variables|Default|SetCanReset? true))))

(event Input|KeyboardEvents|Up
  (params (Key :type Key%20Structure :default "None"))
  (:Pressed
    (Utilities|FlowControl|DoOnce false
      (:Completed
        (Audio|PlaySoundatLocation "/Game/Misc/CarStart.CarStart" (Transformation|GetActorLocation) "0, 0, 0" 2.0 1.0 0.0 "/Game/VehicleAdv/Sound/Engine_att.Engine_att" 0 0)
        (Utilities|FlowControl|Delay 0.7)
        (Components|Activation|Activate (Variables|Default|GetAuto) false)
        (Utilities|FlowControl|Delay 0.2)
        (Variables|Default|SetCarStarted true)))))

(event Input|KeyboardEvents|Down
  (params (Key :type Key%20Structure :default "None"))
  (:Pressed
    (Utilities|FlowControl|DoOnce false
      (:Completed
        (Audio|PlaySoundatLocation "/Game/Misc/CarStart.CarStart" (Transformation|GetActorLocation) "0, 0, 0" 2.0 1.0 0.0 "/Game/VehicleAdv/Sound/Engine_att.Engine_att" 0 0)
        (Utilities|FlowControl|Delay 0.7)
        (Components|Activation|Activate (Variables|Default|GetAuto) false)
        (Utilities|FlowControl|Delay 0.2)
        (Variables|Default|SetCarStarted true)))))

(fn ConstructionScript)